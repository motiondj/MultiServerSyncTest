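; Sync diagnostics logger that samples the first BP_SyncTimeVisualizer actor on a looping timer while logging is enabled.
; Each sample sets arrays for timestamp, time offset, frame number, master/slave state and sync status, replacing previous contents, so the ten-entry trim never accumulates history.
; On EndPlay it optionally builds CSV text and calls a save to a dated Saved-directory path, though the text is not visibly passed to that call.
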(event `self.ReceiveBeginPlay`
  (`KismetArrayLibrary.Array_Clear` (`self.ArrayOfTimestamps`))
  (`KismetArrayLibrary.Array_Clear` (`self.ArrayOfFrameNumbers`))
  (`KismetArrayLibrary.Array_Clear` (`self.ArrayOfNodeStates`))
  (`KismetArrayLibrary.Array_Clear` (`self.ArrayOfSyncStates`))
  (`KismetArrayLibrary.Array_Clear` (`self.ArrayOfTimestamps`))
  (if (`self.LoggingEnabled `)
    (`KismetSystemLibrary.K2_SetTimer` null "LogSyncData" (`self.LogInterval`) true)))

(event `self.ReceiveEndPlay`
  (params (EndPlayReason :type "EEndPlayReason Enum" :default "Destroyed"))
  (`KismetSystemLibrary.K2_ClearTimer` null "LogSyncData")
  (if (`self.SaveToFile`)
    (`self.SaveLogToCSV`)))

(fn `LogSyncData`
  (locals (Master :type String) (Slave :type String))
  (bind _output (`|GetArrayItem` (`self.Out Actors`)))
  (bind _outactors (`GameplayStatics.GetAllActorsOfClass` "/Game/Blueprints/BP_SyncTimeVisualizer.BP_SyncTimeVisualizer_C"))
  (bind _output_get (set `self.Out Actors` _outactors))
  (if (> (`KismetArrayLibrary.Array_Length` _output_get) 0)
    (set `self.ArrayOfTimeOffsets` (`|MakeArray` (`SyncTestActor.GetTimeOffset` _output) :!type "Float (double-precision)"))
    (set `self.ArrayOfFrameNumbers` (`|MakeArray` (`SyncTestActor.GetCurrentFrameNumber` _output)))
    (if (`SyncTestActor.IsMasterNode` _output)
      (bind _output_get_2 (set `local.Master` "Master"))
      (else
        (bind _output_get_3 (set `local.Slave` "Slave"))))
    (set `self.ArrayOfNodeStates` (`|MakeArray` _output_get_2 _output_get_3))
    (set `self.ArrayOfSyncStates` (`|MakeArray` (`SyncTestActor.GetSyncStatusText` _output)))
    (bind _output_get_4 (set `self.ArrayOfTimestamps` (`|MakeArray` (`self.GetGameTimeSinceCreation` _output) :!type "Float (double-precision)")))
    (if (> (`KismetArrayLibrary.Array_Length` _output_get_4) 10)
      (`KismetArrayLibrary.Array_Remove` _output_get_4)
      (`KismetArrayLibrary.Array_Remove` (`self.ArrayOfTimeOffsets`))
      (`KismetArrayLibrary.Array_Remove` (`self.ArrayOfFrameNumbers`))
      (`KismetArrayLibrary.Array_Remove` (`self.ArrayOfNodeStates`))
      (`KismetArrayLibrary.Array_Remove` (`self.ArrayOfSyncStates`)))
    (else
      (return))))

(fn `SaveLogToCSV`
  (bind (_year _month _day) (`KismetMathLibrary.BreakDateTime` (`KismetMathLibrary.Now`)))
  (bind _output_get (set `self.CSV String` "\"Timestamp,TimeOffset,FrameNumber,NodeState,SyncState\\n\""))
  (for _index (range (`KismetArrayLibrary.Array_Length` (`self.ArrayOfTimeOffsets`)))
    (set `self.Index` _index)
    (set `self.CSV String` (`KismetStringLibrary.Concat_StrStr` _output_get (`KismetTextLibrary.Conv_TextToString` (`|FormatText` "\"{0},{1},{2},{4},{5}\\n\"" (`KismetStringLibrary.Conv_DoubleToString` (`|GetArrayItem` (`self.ArrayOfTimestamps`) (`self.Index`))) (`|GetArrayItem` (`self.ArrayOfTimeOffsets`) (`self.Index`)) (`KismetStringLibrary.Conv_IntToString` (`|GetArrayItem` (`self.ArrayOfFrameNumbers`) (`self.Index`))) (`|GetArrayItem` (`self.ArrayOfNodeStates`) (`self.Index`)) (`|GetArrayItem` (`self.ArrayOfSyncStates`) (`self.Index`)))))))
  (`InterchangeBaseNodeContainer.SaveToFile` (`KismetTextLibrary.Conv_TextToString` (`|FormatText` "\"{0}/Synclog_{1}.csv\"" (`KismetSystemLibrary.GetProjectSavedDirectory`) (`KismetStringLibrary.Concat_StrStr` (`KismetStringLibrary.Conv_IntToString` _year) (`KismetStringLibrary.Conv_IntToString` _month) (`KismetStringLibrary.Conv_IntToString` _day)))))
  (`KismetSystemLibrary.PrintString` "\"CSV 저장 완료!\""))

(fn `UserConstructionScript`)