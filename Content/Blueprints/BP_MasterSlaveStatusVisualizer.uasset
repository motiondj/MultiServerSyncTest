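; Status display actor that labels itself as a master or slave node through a text component and a colored mesh.
; CheckMasterStatus uses the ForceMaster flag to set role, status string and dynamic material color, with a random float standing in for time offset.
; UpdateDisplay writes the text only at BeginPlay.
; Tick re-runs the check only when a single frame exceeds half a second, without refreshing the text.
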(event `self.ReceiveBeginPlay`
  (bind _returnvalue (`PrimitiveComponent.CreateDynamicMaterialInstance` (`self.DisplayMesh`) 0 "/Game/Materials/MI_Color_Black.MI_Color_Black" "None"))
  (set `self.DynamicMaterialInstance_Ref` _returnvalue)
  (`self.CheckMasterStatus`)
  (`self.UpdateDisplay `))

(event `self.ReceiveTick`
  (params (DeltaSeconds :type "Float (single-precision)"))
  (if (> DeltaSeconds 0.5)
    (`self.CheckMasterStatus`)))

(fn `CheckMasterStatus`
  (if (`self.bForceMaster `)
    (set `self.IsMasterNode` true)
    (bind _output_get (set `self.StatusColor` (struct :`B` 1.0 :`A` 1.0)))
    (`MaterialInstanceDynamic.SetVectorParameterValue` (`self.DynamicMaterialInstance_Ref`) "Color" _output_get)
    (set `self.Srt_StatusText` "Force Master enabled")
    (else
      (set `self.IsMasterNode` false)
      (bind _output_get_2 (set `self.TimeOffset` (`KismetMathLibrary.RandomFloat`)))
      (if (< _output_get_2 2.0)
        (bind _output_get_3 (set `self.StatusColor` (struct :`R` 1.0 :`B` 1.0 :`A` 1.0)))
        (`MaterialInstanceDynamic.SetVectorParameterValue` (`self.DynamicMaterialInstance_Ref`) "Color" _output_get_3)
        (set `self.Srt_StatusText` "Syncing (<2ms)")
        (else
          (set `self.Srt_StatusText` (`KismetStringLibrary.Concat_StrStr` "Syncing (" (`KismetStringLibrary.Conv_DoubleToString` _output_get_2) " ms)")))))))

(fn `UpdateDisplay `
  (if (`self.bForceMaster `)
    (bind _output_get (set `self.masterslave` "Master Node"))
    (`TextRenderComponent.K2_SetText` (`self.StatusText`) _output_get)
    (else
      (bind _output_get_2 (set `self.masterslave` "Slave Node"))
      (`TextRenderComponent.K2_SetText` (`self.StatusText`) (`|FormatText` "{0} : {1} , Offset : {2}" _output_get_2 (`self.Srt_StatusText`) (`self.TimeOffset`))))))

(fn `UserConstructionScript`)