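; Debug visualizer actor that shows network time sync status in the world through text and a colored mesh.
; Each Tick fires the visualizer event, which writes the time offset and sync status to two text components.
; The mesh turns blue on the master node, otherwise green when in sync and red when out of sync.
; A file logging call is present but unconnected.
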(event `self.ReceiveTick`
  (params (DeltaSeconds :type "Float (single-precision)"))
  (`self.SyncTimeVisualizer_Event`))

(event `SyncTimeVisualizer_Event`
  (`TextRenderComponent.K2_SetText` (`self.TimeOffsetText`) (`KismetTextLibrary.Conv_DoubleToText` (`self.GetTimeOffset`) "HalfToEven"))
  (`TextRenderComponent.K2_SetText` (`self.StatusText`) (`KismetTextLibrary.Conv_StringToText` (`self.GetSyncStatusText`)))
  (if (`self.IsMasterNode`)
    (`PrimitiveComponent.SetMaterial` (`self.VisualizerMesh`) 0 "/Game/Materials/MI_Color_Blue.MI_Color_Blue")
    (elif (`self.IsTimeInSync`)
      (`PrimitiveComponent.SetMaterial` (`self.VisualizerMesh`) 0 "/Game/Materials/MI_Color_Green.MI_Color_Green")
      (else
        (`PrimitiveComponent.SetMaterial` (`self.VisualizerMesh`) 0 "/Game/Materials/MI_Color_Red.MI_Color_Red")))))

(fn `UserConstructionScript`)